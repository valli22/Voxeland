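; Game mode for Voxeland, going by its name, that tracks remaining players and flags a win when one or none is left.
; BeginPlay hard-codes the player count to three, clears the win flag and looks up tagged player controllers, but leaves the controller reference empty.
; LessPlayer decrements the count, and Tick polls it, setting HasWin and printing a debug win message every frame once the condition holds.
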(event `self.ReceiveBeginPlay`
  (set `self.PlayersInGame` 3)
  (bind _outactors (`GameplayStatics.GetAllActorsWithTag` "PlayersController"))
  (set `self.PController` null)
  (set `self.HasWin` false))

(event `self.ReceiveTick`
  (params (DeltaSeconds :type "Float (single-precision)"))
  (if (<= (`self.PlayersInGame`) 1)
    (set `self.HasWin` true)
    (`KismetSystemLibrary.PrintString` "WIN")))

(fn `LessPlayer`
  (set `self.PlayersInGame` (- (`self.PlayersInGame`) 1)))

(fn `UserConstructionScript`)