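; Player controller for Minijuego2 that runs three characters for what appears to be local multiplayer.
; On BeginPlay it spawns two extra controllers and characters at fixed locations and has each controller possess its character.
; This controller still handles all input, routing separate move and jump mappings to its own pawn and the two stored character references.
; Movement follows fixed world X/Y axes, independent of camera or control rotation.
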(event `self.ReceiveBeginPlay`
  (bind _returnvalue (`KismetMathLibrary.MakeTransform` (-1100.0 -1376.0 232.0)))
  (bind _returnvalue_2 (`KismetMathLibrary.MakeTransform` (-1000.0 -1376.0 232.0)))
  (bind _returnvalue_3 (`|SpawnActorFromClass` "/Game/Voxeland/Blueprints/SpeedRun/MyPlayerController2.MyPlayerController2_C" _returnvalue_2 "Undefined" "OverrideRootScale" null null))
  (set `self.controller2` _returnvalue_3)
  (bind _returnvalue_4 (`|SpawnActorFromClass` "/Game/Voxeland/Blueprints/SpeedRun/Character2_BP.Character2_BP_C" _returnvalue_2 "Undefined" "OverrideRootScale" null null))
  (set `self.character2` _returnvalue_4)
  (`self.Possess` (`self.controller2`) (`self.character2`))
  (bind _returnvalue_5 (`|SpawnActorFromClass` "/Game/Voxeland/Blueprints/SpeedRun/MyPlayerController3.MyPlayerController3_C" _returnvalue "Undefined" "OverrideRootScale" null null))
  (set `self.controller3` _returnvalue_5)
  (bind _returnvalue_6 (`|SpawnActorFromClass` "/Game/Voxeland/Blueprints/SpeedRun/Character3_BP.Character3_BP_C" _returnvalue "Undefined" "OverrideRootScale" null null))
  (set `self.character3` _returnvalue_6)
  (`self.Possess` (`self.controller3`) (`self.character3`)))

(event `InputAxis|MoveRight`
  (params (AxisValue :type "Float (single-precision)"))
  (`Pawn.AddMovementInput` (`self.K2_GetPawn`) (0.0 10.0 0.0) AxisValue false))

(event `InputAction|Action`
  (params (Key :type "Key Structure"))
  (:`Pressed`
    (`Character.Jump` (`GameplayStatics.GetPlayerCharacter` 0))))

(event `InputAxis|MoveForward`
  (params (AxisValue :type "Float (single-precision)"))
  (`Pawn.AddMovementInput` (`self.K2_GetPawn`) (10.0 0.0 0.0) AxisValue false))

(event `InputAction|Action2`
  (params (Key :type "Key Structure"))
  (:`Pressed`
    (`Character.Jump` (`self.character2`))))

(event `InputAxis|MoveRight2`
  (params (AxisValue :type "Float (single-precision)"))
  (`Pawn.AddMovementInput` (`self.character2`) (0.0 10.0 0.0) AxisValue false))

(event `InputAxis|MoveForward2`
  (params (AxisValue :type "Float (single-precision)"))
  (`Pawn.AddMovementInput` (`self.character2`) (10.0 0.0 0.0) AxisValue false))

(event `InputAxis|MoveForward3`
  (params (AxisValue :type "Float (single-precision)"))
  (`Pawn.AddMovementInput` (`self.character3`) (10.0 0.0 0.0) AxisValue false))

(event `InputAction|Action3`
  (params (Key :type "Key Structure"))
  (:`Pressed`
    (`Character.Jump` (`self.character3`))))

(event `InputAxis|MoveRight3`
  (params (AxisValue :type "Float (single-precision)"))
  (`Pawn.AddMovementInput` (`self.character3`) (0.0 10.0 0.0) AxisValue false))

(fn `UserConstructionScript`)