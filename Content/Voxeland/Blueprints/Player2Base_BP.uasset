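; Base Blueprint for the second player in Voxeland, providing axis-driven movement along world X and Y.
; On BeginPlay it creates a player with controller ID 1 and sets a fixed Velocity value.
; P2UpDown and P2RightLeft apply movement input outside a small dead zone, using only the axis sign for direction and Velocity as the scale, so input is not analog.
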(event `self.ReceiveBeginPlay`
  (`GameplayStatics.CreatePlayer` 1)
  (set `self.Velocity` 500.0))

(event `InputAxis|P2UpDown`
  (params (AxisValue :type "Float (single-precision)"))
  (if (> AxisValue 0.1)
    (`self.AddMovementInput` (1.0 0.0 0.0) (`self.Velocity`))
    (elif (< AxisValue -0.1)
      (`self.AddMovementInput` (-1.0 0.0 0.0) (`self.Velocity`)))))

(event `InputAxis|P2RightLeft`
  (params (AxisValue :type "Float (single-precision)"))
  (if (> AxisValue 0.1)
    (`self.AddMovementInput` (0.0 1.0 0.0) (`self.Velocity`))
    (elif (< AxisValue -0.1)
      (`self.AddMovementInput` (0.0 -1.0 0.0) (`self.Velocity`)))))

(fn `UserConstructionScript`)