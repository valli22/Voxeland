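; Camera_BP is a speed-run camera actor that follows the leading player along the world Y axis.
; On BeginPlay it caches the first MyPlayerController, which also references Controller2 and Controller3.
; Each Tick it compares the three controlled pawns' Y positions, picks the largest, and moves its scene component there, keeping X and Z unchanged.
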(event `self.ReceiveBeginPlay`
  (bind _outactors (`GameplayStatics.GetAllActorsOfClass` "/Game/Voxeland/Blueprints/SpeedRun/MyPlayerController.MyPlayerController_C"))
  (set `self.Actor` (`|GetArrayItem` _outactors)))

(event `self.ReceiveTick`
  (params (DeltaSeconds :type "Float (single-precision)"))
  (bind _scenecomponent (`self.SceneComponent`))
  (bind _y (.y (`self.K2_GetActorLocation` (`Controller.K2_GetPawn` (`self.Actor`)))))
  (bind _y_2 (.y (`self.K2_GetActorLocation` (`Controller.K2_GetPawn` (`/Game/Voxeland/Blueprints/SpeedRun/MyPlayerController.controller2` (`self.Actor`))))))
  (bind _y_3 (.y (`self.K2_GetActorLocation` (`Controller.K2_GetPawn` (`/Game/Voxeland/Blueprints/SpeedRun/MyPlayerController.controller3` (`self.Actor`))))))
  (if (>= _y _y_2)
    (if (>= _y _y_3)
      (set `self.yObjective` _y)
      (else
        (set `self.yObjective` _y_3 :!label _label)))
    (elif (>= _y_2 _y_3)
      (set `self.yObjective` _y_2)
      (else
        (goto _label))))
  (`SceneComponent.K2_SetWorldLocation` _scenecomponent (`KismetMathLibrary.MakeVector` (.x (`SceneComponent.K2_GetComponentLocation` _scenecomponent)) (`self.yObjective`) (.z (`SceneComponent.K2_GetComponentLocation` _scenecomponent))) false false))

(fn `UserConstructionScript`)