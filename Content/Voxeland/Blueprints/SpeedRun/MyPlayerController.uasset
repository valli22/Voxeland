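; Player controller for the SpeedRun mode that drives three auto-running characters from one set of inputs.
; On BeginPlay it spawns two extra controllers and characters, possesses them, and locks all movement until the StartOurGame input.
; Once started, Tick pushes each character along +Y at RunSpeed, while per-character axis and action inputs handle X-axis movement and jumping.
; Inputs for all three are handled here and forwarded directly to the pawns, gated by separate CanMove flags.
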(event `InputAction|StartOurGame`
  (params (Key :type "Key Structure"))
  (:`Pressed`
    (if (not (`self.HasStarted`))
      (set `self.canMove1` true)
      (set `self.canMove2` true)
      (set `self.canMove3` true)
      (set `self.HasStarted` true))))

(event `self.ReceiveBeginPlay`
  (bind _returnvalue (`KismetMathLibrary.MakeTransform` (-1100.0 -1376.0 232.0)))
  (bind _returnvalue_2 (`KismetMathLibrary.MakeTransform` (-1000.0 -1376.0 232.0)))
  (bind _returnvalue_3 (`|SpawnActorFromClass` "/Game/Voxeland/Blueprints/SpeedRun/MyPlayerController2.MyPlayerController2_C" _returnvalue_2 "Undefined" "OverrideRootScale" null null))
  (set `self.controller2` _returnvalue_3)
  (bind _returnvalue_4 (`|SpawnActorFromClass` "/Game/Voxeland/Blueprints/SpeedRun/Character2_BP.Character2_BP_C" _returnvalue_2 "Undefined" "OverrideRootScale" null null))
  (set `self.character2` _returnvalue_4)
  (`self.Possess` (`self.controller2`) (`self.character2`))
  (bind _returnvalue_5 (`|SpawnActorFromClass` "/Game/Voxeland/Blueprints/SpeedRun/MyPlayerController3.MyPlayerController3_C" _returnvalue "Undefined" "OverrideRootScale" null null))
  (set `self.controller3` _returnvalue_5)
  (bind _returnvalue_6 (`|SpawnActorFromClass` "/Game/Voxeland/Blueprints/SpeedRun/Character3_BP.Character3_BP_C" _returnvalue "Undefined" "OverrideRootScale" null null))
  (set `self.character3` _returnvalue_6)
  (`self.Possess` (`self.controller3`) (`self.character3`))
  (set `self.RunSpeed` 1.0)
  (set `self.canMove1` false)
  (set `self.canMove2` false)
  (set `self.canMove3` false)
  (set `self.HasStarted` false))

(event `InputAction|Action`
  (params (Key :type "Key Structure"))
  (:`Pressed`
    (if (`self.canMove1`)
      (`Character.Jump` (`GameplayStatics.GetPlayerCharacter` 0)))))

(event `InputAxis|MoveForward`
  (params (AxisValue :type "Float (single-precision)"))
  (if (`self.canMove1`)
    (`Pawn.AddMovementInput` (`self.K2_GetPawn`) (10.0 0.0 0.0) AxisValue false)))

(event `InputAction|Action2`
  (params (Key :type "Key Structure"))
  (:`Pressed`
    (if (`self.canMove2`)
      (`Character.Jump` (`self.character2`)))))

(event `InputAxis|MoveForward2`
  (params (AxisValue :type "Float (single-precision)"))
  (if (`self.canMove2`)
    (`Pawn.AddMovementInput` (`self.character2`) (10.0 0.0 0.0) AxisValue false)))

(event `InputAxis|MoveForward3`
  (params (AxisValue :type "Float (single-precision)"))
  (if (`self.canMove3`)
    (`Pawn.AddMovementInput` (`self.character3`) (10.0 0.0 0.0) AxisValue false)))

(event `InputAction|Action3`
  (params (Key :type "Key Structure"))
  (:`Pressed`
    (if (`self.canMove3`)
      (`Character.Jump` (`self.character3`)))))

(event `self.ReceiveTick`
  (params (DeltaSeconds :type "Float (single-precision)"))
  (bind _runspeed (`self.RunSpeed`))
  (if (`self.canMove1`)
    (`Pawn.AddMovementInput` (`self.K2_GetPawn`) (0.0 10.0 0.0) _runspeed false))
  (if (`self.canMove2`)
    (`Pawn.AddMovementInput` (`self.character2`) (0.0 10.0 0.0) _runspeed false))
  (if (`self.canMove3`)
    (`Pawn.AddMovementInput` (`self.character3`) (0.0 10.0 0.0) _runspeed false)))

(fn `UserConstructionScript`)