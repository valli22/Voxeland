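; Win trigger for the Voxeland SpeedRun mode that declares whichever tagged player overlaps it as the last one in play.
; BeginPlay caches a single MyPlayerController found by the "PlayersController" tag.
; Any overlap plays a scream sound, then the actor's first tag (Player1–3) selects which other two players lose their CanMove flags.
; A matched player also sets PlayersInGame to 1 on VoxelandGM_BP.
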(event `self.ReceiveBeginPlay`
  (bind _outactors (`GameplayStatics.GetAllActorsWithTag` "PlayersController"))
  (bind _asmy_player_controller (cast `/Game/Voxeland/Blueprints/SpeedRun/MyPlayerController` (`|GetArrayItem` _outactors)))
  (set `self.playerController` _asmy_player_controller))

(event `self.ReceiveActorBeginOverlap`
  (params (OtherActor :type "Actor Object Reference"))
  (bind _playercontroller (`self.playerController`))
  (bind _output (`|GetArrayItem` (`Actor.Tags` OtherActor)))
  (`GameplayStatics.PlaySound2D` "/Game/Voxeland/Sounds/348310__redafs__zombie-monster-scream.348310__redafs__zombie-monster-scream")
  ;[1 1 1] Old technique
  (if (== _output "Player1")
    (set `/Game/Voxeland/Blueprints/SpeedRun/MyPlayerController.canMove2` false _playercontroller)
    (set `/Game/Voxeland/Blueprints/SpeedRun/MyPlayerController.canMove3` false _playercontroller)
    (bind _asvoxeland_gm_bp (cast `/Game/Voxeland/Blueprints/VoxelandGM_BP` (`GameplayStatics.GetGameMode`) :!label _label))
    (set `/Game/Voxeland/Blueprints/VoxelandGM_BP.PlayersInGame` 1 _asvoxeland_gm_bp)
    (elif (== _output "Player2")
      (set `/Game/Voxeland/Blueprints/SpeedRun/MyPlayerController.canMove1` false _playercontroller)
      (set `/Game/Voxeland/Blueprints/SpeedRun/MyPlayerController.canMove3` false _playercontroller)
      (goto _label)
      (elif (== _output "Player3")
        (set `/Game/Voxeland/Blueprints/SpeedRun/MyPlayerController.canMove1` false _playercontroller)
        (set `/Game/Voxeland/Blueprints/SpeedRun/MyPlayerController.canMove2` false _playercontroller)
        (goto _label)))))

(fn `UserConstructionScript`)