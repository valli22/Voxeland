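; Death zone actor for the SpeedRun mode that eliminates players who fall behind the camera.
; Each tick it moves its collision component along Y to trail the player camera at a fixed offset.
; An overlapping actor tagged Player1, Player2 or Player3 has its movement flag cleared on the tag-located MyPlayerController, then the VoxelandGM_BP game mode's LessPlayer is called.
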(event `self.ReceiveBeginPlay`
  (bind _outactors (`GameplayStatics.GetAllActorsWithTag` "PlayersController"))
  (bind _asmy_player_controller (cast `/Game/Voxeland/Blueprints/SpeedRun/MyPlayerController` (`|GetArrayItem` _outactors)))
  (set `self.playerController` _asmy_player_controller))

(event `self.ReceiveActorBeginOverlap`
  (params (OtherActor :type "Actor Object Reference"))
  (bind _playercontroller (`self.playerController`))
  (bind _output (`|GetArrayItem` (`Actor.Tags` OtherActor)))
  (if (== _output "Player1")
    (set `/Game/Voxeland/Blueprints/SpeedRun/MyPlayerController.canMove1` false _playercontroller)
    (bind _asvoxeland_gm_bp (cast `/Game/Voxeland/Blueprints/VoxelandGM_BP` (`GameplayStatics.GetGameMode`) :!label _label))
    (`/Game/Voxeland/Blueprints/VoxelandGM_BP.LessPlayer` _asvoxeland_gm_bp)
    (elif (== _output "Player2")
      (set `/Game/Voxeland/Blueprints/SpeedRun/MyPlayerController.canMove2` false _playercontroller)
      (goto _label)
      (elif (== _output "Player3")
        (set `/Game/Voxeland/Blueprints/SpeedRun/MyPlayerController.canMove3` false _playercontroller)
        (goto _label)))))

(event `self.ReceiveTick`
  (params (DeltaSeconds :type "Float (single-precision)"))
  (`SceneComponent.K2_SetWorldLocation` (`self.CollisionComponent`) (`KismetMathLibrary.MakeVector` (.x (`SceneComponent.K2_GetComponentLocation` (`self.CollisionComponent`))) (- (.y (`self.K2_GetActorLocation` (`GameplayStatics.GetPlayerCameraManager` 0))) 873.0) (.z (`SceneComponent.K2_GetComponentLocation` (`self.CollisionComponent`)))) false false))

(fn `UserConstructionScript`)