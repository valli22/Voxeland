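; Second character Blueprint for the SpeedRun mode, handling damage and death.
; AnyDamage subtracts from Health and hides one UI image on a non-lethal hit, reaching the widget through the SpeedRun HUD.
; At zero or below, it disables CanMove2 on player controller 0, sets RIP, calls LessPlayer on the game mode and hides both images.
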(event `self.ReceiveAnyDamage`
  (params (Damage :type "Float (single-precision)") (DamageType :type "DamageType Object Reference") (InstigatedBy :type "Controller Object Reference") (DamageCauser :type "Actor Object Reference"))
  (bind _returnvalue (- (`self.Health`) Damage))
  (if (<= _returnvalue 0.0)
    (set `self.Health` _returnvalue)
    (bind _asmy_player_controller (cast `/Game/Voxeland/Blueprints/SpeedRun/MyPlayerController` (`GameplayStatics.GetPlayerController` 0)))
    (set `/Game/Voxeland/Blueprints/SpeedRun/MyPlayerController.canMove2` false _asmy_player_controller)
    (set `self.RIP` true)
    (bind _asvoxeland_gm_bp (cast `/Game/Voxeland/Blueprints/VoxelandGM_BP` (`GameplayStatics.GetGameMode`)))
    (`/Game/Voxeland/Blueprints/VoxelandGM_BP.LessPlayer` _asvoxeland_gm_bp)
    (bind _asspeed_run_hudclass_bp (cast `/Game/Voxeland/Blueprints/SpeedRun/SpeedRunHUDClass_BP` (`PlayerController.GetHUD` (`GameplayStatics.GetPlayerController` 0))))
    (bind _asui_bp (cast `/Game/Voxeland/Blueprints/SpeedRun/UI_BP` (`/Game/Voxeland/Blueprints/SpeedRun/SpeedRunHUDClass_BP.UI Widget` _asspeed_run_hudclass_bp)))
    (`Image.SetOpacity` (`/Game/Voxeland/Blueprints/SpeedRun/UI_BP.Image_188` _asui_bp) 0.0)
    (`Image.SetOpacity` (`/Game/Voxeland/Blueprints/SpeedRun/UI_BP.Image_189` _asui_bp) 0.0)
    (else
      (set `self.Health` _returnvalue)
      (bind _asspeed_run_hudclass_bp_2 (cast `/Game/Voxeland/Blueprints/SpeedRun/SpeedRunHUDClass_BP` (`PlayerController.GetHUD` (`GameplayStatics.GetPlayerController` 0))))
      (bind _asui_bp_2 (cast `/Game/Voxeland/Blueprints/SpeedRun/UI_BP` (`/Game/Voxeland/Blueprints/SpeedRun/SpeedRunHUDClass_BP.UI Widget` _asspeed_run_hudclass_bp_2)))
      (`Image.SetOpacity` (`/Game/Voxeland/Blueprints/SpeedRun/UI_BP.Image_189` _asui_bp_2) 0.0))))

(fn `UserConstructionScript`)